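; Blueprint function library of helper checks for inventory slots.
; IsSlotEmpty treats a slot as empty when its Item does not resolve to a valid object.
; IsStackableAndHaveSpace rejects empty target slots, then queries the target item through an IsItemStackable message.
; It returns the stack size and whether the item is stackable, shares the incoming slot's ItemID and has quantity below that size.
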(fn `IsSlotEmpty`
  (params (Slot :type "InventoryItemTypes Structure"))
  (returns (Success :type Boolean))
  (return (not (`KismetSystemLibrary.IsValid` (`|ConvertAsset` (`.Item` (break `InventoryItemTypes` Slot)))))))

(fn `IsStackableAndHaveSpace`
  (params (TargetSlot :type "InventoryItemTypes Structure (by ref)") (SlotToStack :type "InventoryItemTypes Structure (by ref)"))
  (returns (Result :type Boolean) (ItemStackSize :type Integer))
  (bind ((`ItemID` _itemid) (`Quantity` _quantity) (`Item` _item)) (break `InventoryItemTypes` TargetSlot))
  (if (`self.IsSlotEmpty` TargetSlot)
    (return false 0)
    (else
      (bind _returnvalue (message `C_InventoryAssetInterface.IsItemStackable` (`|ConvertAsset` _item)))
      (bind (_isstackable _stacksize) (break `StackableResult` _returnvalue))
      (return (and _isstackable (== _itemid (`.ItemID` (break `InventoryItemTypes` SlotToStack))) (< _quantity _stacksize)) _stacksize))))