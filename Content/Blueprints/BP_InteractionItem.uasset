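; BP_InteractionItem is a world item that the player picks up by interacting with it.
; On Interact, it gets the item's ID through GetItemIDMessage and passes it, with the quantity and item reference, to AddItem on the first player character's BP_InventoryComponent.
; It then destroys itself without checking whether the add succeeded.
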(event `Interact`
  (bind _returnvalue (message `C_InventoryAssetInterface.GetItemID` (`self.Item`)))
  (`/UE5_InventorySystem/Blueprints/BP_InventoryComponent.BP_AddItem` (`self.GetComponentByClass` (`GameplayStatics.GetPlayerCharacter` 0) "/UE5_InventorySystem/Blueprints/BP_InventoryComponent.BP_InventoryComponent_C") _returnvalue (`self.Quantity`) (`self.Item`))
  (`self.K2_DestroyActor`))

(fn `UserConstructionScript`
  (`parent.UserConstructionScript`))