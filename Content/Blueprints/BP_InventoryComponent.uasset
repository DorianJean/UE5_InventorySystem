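; Slot-based inventory component that stores items, opens the inventory widget on Tab and interacts with BP_InteractionItem actors through a camera line trace on E.
; AddItem tops up stackable slots, then splits the remainder across empty slots, with a pickup sound on full success.
; TransferItem moves items within or between components through AddItemToIndex, which fills, stacks or swaps slots.
; Transfers without a target index are still a TODO.
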(event `self.ReceiveBeginPlay`
  (`self.SetupSlots` (`self.MaxInventoryAmount`)))

(event `BP_AddItem`
  (params (`Item ID` :type Name) (Quantity :type Integer) (Item :type "C_InventoryItemInfo Object Reference"))
  (bind _success (`self.AddItem` (make `InventoryItemTypes` :`ItemID` `Item ID` :`Quantity` Quantity :`Item` (`|ConvertAsset` Item))))
  (if _success
    (`GameplayStatics.PlaySound2D` (`C_InventoryItemInfo.PickupSound` Item) 1.0 1.0 0.0 null null)))

(event `BP_TransferItem`
  (params (ToInventoryComponent :type "/Game/Blueprints/BP_InventoryComponent Object Reference") (FromIndex :type Integer) (ToIndex :type Integer))
  (`self.TransferItem` ToInventoryComponent FromIndex ToIndex))

(event `Key|Tab`
  (params (Key :type "Key Structure"))
  (:`Pressed`
    (`self.ToggleInventory` true)))

(event `Key|E`
  (params (Key :type "Key Structure"))
  (bind _rootcomponent (`Actor.RootComponent` (`GameplayStatics.GetPlayerCameraManager` 0)))
  (bind _returnvalue (`SceneComponent.K2_GetComponentLocation` _rootcomponent))
  (:`Pressed`
    (bind _outhit (`KismetSystemLibrary.LineTraceSingle` _returnvalue (+ _returnvalue (* (`KismetMathLibrary.GetForwardVector` (`SceneComponent.K2_GetComponentRotation` _rootcomponent)) 500.0)) "TraceTypeQuery1"))
    (bind _asbp_interaction_item (cast `/UE5_InventorySystem/Blueprints/BP_InteractionItem` (`.HitActor` (`GameplayStatics.BreakHitResult` _outhit))))
    (`/UE5_InventorySystem/Blueprints/BP_InteractionItem.Interact` _asbp_interaction_item)))

(fn `AddItem`
  (params (ItemToAdd :type "InventoryItemTypes Structure"))
  (returns (Success :type Boolean))
  (locals (ItemStackSize :type Integer :default 0) (NewQuantityFromTargetSlot :type Integer) (CurrentItemToAdd :type "InventoryItemTypes Structure") (TargetSlot :type "InventoryItemTypes Structure") (TemporaryCacheItemToAdd :type "InventoryItemTypes Structure"))
  (bind _currentitemtoadd (`local.CurrentItemToAdd`))
  (bind _output_get (set `local.CurrentItemToAdd` ItemToAdd))
  (bind _returnvalue (message `C_InventoryAssetInterface.IsItemStackable` (`|ConvertAsset` (`.Item` (break `InventoryItemTypes` _output_get)))))
  (bind (_isstackable _stacksize) (break `StackableResult` _returnvalue))
  (set `local.ItemStackSize` _stacksize)
  (if _isstackable
    (for _array_element (`self.InventoryItemList`)
      (bind _output_get_2 (set `local.TargetSlot` _array_element))
      (if (`/UE5_InventorySystem/Blueprints/BFL_InventoryFunctionLibrary.IsStackableAndHaveSpace` _output_get_2 _currentitemtoadd)
        (bind _output_get_3 (set `local.NewQuantityFromTargetSlot` (+ (`.Quantity` (break `InventoryItemTypes` _array_element)) (`.Quantity` (break `InventoryItemTypes` _currentitemtoadd)))))
        (if (> _output_get_3 (`local.ItemStackSize`))
          (`self.SetQuantityAtSlot` (`local.TargetSlot`) (`local.ItemStackSize`))
          (setmembers `InventoryItemTypes` :`StructRef` (`local.CurrentItemToAdd`) :`Quantity` (- (`local.NewQuantityFromTargetSlot`) (`local.ItemStackSize`)))
          (else
            (`self.SetQuantityAtSlot` (`local.TargetSlot`) (`local.NewQuantityFromTargetSlot`))
            (return true))))))
  ; Add Item To Empty Slots
  (bind (_slot _index _returnvalue_2) (`self.FindEmptySlot` :!label _label))
  (if _returnvalue_2
    (set `local.TargetSlot` _slot)
    (if (<= (`.Quantity` (break `InventoryItemTypes` (`local.CurrentItemToAdd`))) (`local.ItemStackSize`))
      (`self.SetItem` (`local.TargetSlot`) (`local.CurrentItemToAdd`))
      (return true)
      (else
        (bind _output_get_4 (set `local.TemporaryCacheItemToAdd` (`local.CurrentItemToAdd`)))
        (bind _structout (setmembers `InventoryItemTypes` :`StructRef` _output_get_4 :`Quantity` (`local.ItemStackSize`)))
        (`self.SetItem` (`local.TargetSlot`) _structout)
        (setmembers `InventoryItemTypes` :`StructRef` (`local.CurrentItemToAdd`) :`Quantity` (- (`.Quantity` (break `InventoryItemTypes` (`local.CurrentItemToAdd`))) (`local.ItemStackSize`)))
        (goto _label)))
    (else
      (`KismetSystemLibrary.PrintString` "Inventory is Full!")
      (return false))))

(fn `AddItemToIndex`
  (params (TargetIndex :type Integer) (ItemSlotToAdd :type "InventoryItemTypes Structure"))
  (returns (Success :type Boolean) (AreAllItemsAdded :type Boolean))
  (bind (_slot _returnvalue) (`self.GetSlotIndex` TargetIndex))
  (bind _itemslottoadd (`local.ItemSlotToAdd`))
  (if _returnvalue
    (if (`/UE5_InventorySystem/Blueprints/BFL_InventoryFunctionLibrary.IsSlotEmpty` _slot)
      (`self.SetItem` _slot _itemslottoadd)
      (return true true)
      (else
        (bind _areallitemsadded (`self.StackItemOnTransfer` _slot _itemslottoadd))
        (return true _areallitemsadded)))
    (else
      (return false false))))

(fn `StackItemOnTransfer`
  (params (TargetSlot :type "InventoryItemTypes Structure") (FromSlot :type "InventoryItemTypes Structure"))
  (returns (AreAllItemsAdded :type Boolean))
  (locals (ItemStackSize :type Integer) (NewQuantityFromTargetSlot :type Integer))
  (bind (_result _itemstacksize) (`/UE5_InventorySystem/Blueprints/BFL_InventoryFunctionLibrary.IsStackableAndHaveSpace` TargetSlot FromSlot))
  (if _result
    (set `local.ItemStackSize` _itemstacksize)
    (bind _output_get (set `local.NewQuantityFromTargetSlot` (+ (`.Quantity` (break `InventoryItemTypes` TargetSlot)) (`.Quantity` (break `InventoryItemTypes` FromSlot)))))
    (if (> _output_get (`local.ItemStackSize`))
      (`self.SetQuantityAtSlot` (`local.TargetSlot`) (`local.ItemStackSize`))
      (`self.SetQuantityAtSlot` (`.InventoryRef` (break `InventoryItemTypes` (`local.FromSlot`))) (`local.FromSlot`) (- (`local.NewQuantityFromTargetSlot`) (`local.ItemStackSize`)))
      (return false)
      (else
        (`self.SetQuantityAtSlot` (`local.TargetSlot`) (`local.NewQuantityFromTargetSlot`))
        (return true)))
    (else
      ; Swap Indexes
      (`self.SwapIndexes` (`local.TargetSlot`) (`local.FromSlot`))
      (return false))))

(fn `ToggleInventory`
  (params (`Activate?` :type Boolean))
  (bind _returnvalue (`GameplayStatics.GetPlayerController` 0))
  (bind _returnvalue_2 (`GameplayStatics.GetPlayerController` 0))
  (if `Activate?`
    (bind _inventoryref (`self.InventoryRef`)
      (:`then`
        (`Widget.RemoveFromParent` _inventoryref))
      (:`else`
        _))
    (bind _returnvalue_3 (`|CreateWidget` "/UE5_InventorySystem/UI/WB_Inventory.WB_Inventory_C"))
    (bind _output_get (set `self.InventoryRef` _returnvalue_3))
    (`/UE5_InventorySystem/UI/WB_Inventory.UpdateInventory` _output_get)
    (`UserWidget.AddToViewport` _output_get 0)
    (`WidgetBlueprintLibrary.SetInputMode_UIOnlyEx` _returnvalue_2 (`self.InventoryRef`))
    (set `PlayerController.bShowMouseCursor` true _returnvalue_2)
    (else
      (bind _inventoryref_2 (`self.InventoryRef`)
        (:`then`
          (`Widget.RemoveFromParent` _inventoryref_2))
        (:`else`
          _))
      (set `self.InventoryRef` null)
      (`WidgetBlueprintLibrary.SetInputMode_GameOnly` _returnvalue)
      (set `PlayerController.bShowMouseCursor` false _returnvalue))))

(fn `TransferItem`
  (params (ToInventoryComponent :type "/Game/Blueprints/BP_InventoryComponent Object Reference") (FromIndex :type Integer) (ToIndex :type Integer))
  (returns (Success :type Boolean))
  (bind _toindex (`local.ToIndex`))
  (if (and (== self ToInventoryComponent) (== FromIndex ToIndex))
    (`KismetSystemLibrary.PrintString` "Error: Same Container & same Slot")
    (return false)
    (elif (and (`KismetSystemLibrary.IsValid` (`local.ToInventoryComponent`)) (`.ReturnValue` (`self.GetSlotIndex` (`local.FromIndex`))) (or (`.ReturnValue` (`self.GetSlotIndex` (`local.ToInventoryComponent`) _toindex)) (== _toindex -1)))
      (if (== (`local.ToIndex`) -1)
        (`KismetSystemLibrary.PrintString` "TODO: Target Slot Index is not specified")
        (else
          (bind (_success _areallitemsadded) (`self.AddItemToIndex` (`local.ToInventoryComponent`) (`local.ToIndex`) (`self.GetSlotIndex` (`local.FromIndex`))))
          (if _success
            (if _areallitemsadded
              (bind _returnvalue (`self.RemoveItemFromIndex` (`local.FromIndex`)))
              (return _returnvalue)
              (else
                (return true)))
            (else
              (return false)))))
      (else
        (return false)))))