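; BP_InventoryItem is an actor that visually represents an inventory item in the world, taking its mesh from its Item reference.
; The construction script calls UpdateItemMesh, which assigns the item's static mesh if valid, otherwise clears that component and falls back to the skeletal mesh.
; Whichever mesh it assigns gets query and physics collision.
; The event graph holds only disabled stub events.
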(fn `UpdateItemMesh`
  (bind _staticmesh (`C_InventoryItemInfo.StaticMesh` (`self.Item`)))
  (bind _skeletalmesh (`C_InventoryItemInfo.SkeletalMesh` (`self.Item`)))
  (`self.Item`
    (:`then`
      (`/Engine/EditorBlueprintResources/StandardMacros.IsValid` _staticmesh
        (:`Is Valid`
          (`StaticMeshComponent.SetStaticMesh` (`self.StaticMesh`) _staticmesh)
          (`PrimitiveComponent.SetCollisionEnabled` (`self.StaticMesh`) "QueryAndPhysics"))
        (:`Is Not Valid`
          (`StaticMeshComponent.SetStaticMesh` (`self.StaticMesh`) null)
          (`/Engine/EditorBlueprintResources/StandardMacros.IsValid` _skeletalmesh
            (:`Is Valid`
              (`SkeletalMeshComponent.SetSkeletalMeshAsset` (`self.SkeletalMesh`) _skeletalmesh)
              (`PrimitiveComponent.SetCollisionEnabled` (`self.SkeletalMesh`) "QueryAndPhysics"))))))
    (:`else`)))

(fn `UserConstructionScript`
  (`self.UpdateItemMesh`))